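; TestPlate_BP is an interactive test plate that tallies the mass of actors resting in its Box trigger.
; An overlap starts a one-second looping CalculateMass timer, which pauses when the box is empty.
; Each tick adds the player pawn's box mass or other actors' static mesh mass to TotalMass, which never resets.
; Results only print to screen; no plate action is implemented.
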(event OnComponentBeginOverlap(Box)
  (params (OverlappedComponent :type Primitive%20Component%20Object%20Reference) (OtherActor :type Actor%20Object%20Reference) (OtherComp :type Primitive%20Component%20Object%20Reference) (OtherBodyIndex :type Integer) (bFromSweep :type Boolean) (SweepResult :type Hit%20Result%20Structure%20%28by%20ref%29))
  (CallFunction|GetTotalMass))

(event Custom|GetTotalMass
  (Utilities|Time|SetTimerbyFunctionName 0 "CalculateMass" 1.0 true))

(event EventBeginPlay)

(event Collision|EventActorBeginOverlap
  (params (OtherActor :type Actor%20Object%20Reference)))

(event EventTick
  (params (DeltaSeconds :type Float%20%28single-precision%29)))

(fn ConstructionScript)

(fn CalculateMass
  (bind _box (Variables|Default|GetBox))
  (bind _overlappingactors (Collision|GetOverlappingActors _box 0 :!class /Script/Engine.PrimitiveComponent))
  (if (> (Utilities|Array|Length _overlappingactors) 0)
    (for _array_element _overlappingactors
      (if (.bSuccess (Utilities|Casting|CastToIllusion_PlayerPawn _array_element))
        (LocalVariables|SetTotalMass (+ (LocalVariables|GetTotalMass) (Physics|GetMass (Actor|GetComponentbyClass (.AsIllusion%20Player%20Pawn (Utilities|Casting|CastToIllusion_PlayerPawn _array_element)) "/Script/Engine.BoxComponent"))))
        (else
          (LocalVariables|SetTotalMass (+ (LocalVariables|GetTotalMass) (Physics|GetMass (Actor|GetComponentbyClass _array_element "/Script/Engine.StaticMeshComponent"))))))
      (Development|PrintString (Utilities|String|Append "Mass ISSSS   " (Utilities|String|ToString(Float) (LocalVariables|GetTotalMass)))))
    (else
      (Development|PrintString "STOP Action from Plate")
      (Class|KismetSystemLibrary|PauseTimer 0 "CalculateMass"))))