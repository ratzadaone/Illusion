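; Test interactive object that flashes its material color once at begin play and can be levitated through telekinesis.
; On BeginPlay it creates a dynamic material instance and uses two chained timelines to lerp the DaColor parameter to a temporary color and back.
; Its Telekinesys event passes the actor to Levitate on the Illusion_PlayerController.
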(event OnBeginCursorOver(StaticMesh)
  (params (TouchedComponent :type Primitive%20Component%20Object%20Reference)))

(event EventBeginPlay
  (bind _returnvalue (Rendering|Material|CreateDynamicMaterialInstance (Variables|Default|GetStaticMesh) 0 "/Game/Materials/TestMat.TestMat" :!class /Script/Engine.PrimitiveComponent))
  (bind _returnvalue_2 (Rendering|Material|GetVectorParameterValue _returnvalue "DaColor" :!class /Script/Engine.MaterialInstanceDynamic))
  (bind _output_get (Variables|Default|SetOrigColor _returnvalue_2))
  (bind _newtrack_0 (Timeline|Timeline_0 PlayFromStart)
    (:Update
      (Rendering|Material|SetVectorParameterValue _returnvalue "DaColor" (Math|Color|Lerp(LinearColor) _output_get (Variables|Default|GetTempColorToChange) _newtrack_0) :!class /Script/Engine.MaterialInstanceDynamic))
    (:Finished
      (bind _newtrack_0_2 (Timeline|Timeline_1 PlayFromStart)
        (:Update
          (Rendering|Material|SetVectorParameterValue _returnvalue "DaColor" (Math|Color|Lerp(LinearColor) (Variables|Default|GetTempColorToChange) (Variables|Default|GetOrigColor) _newtrack_0_2) :!class /Script/Engine.MaterialInstanceDynamic))))))

(event Collision|EventActorBeginOverlap
  (params (OtherActor :type Actor%20Object%20Reference)))

(event EventTick
  (params (DeltaSeconds :type Float%20%28single-precision%29)))

(event EventTelekinesys
  (params (OnOff :type Boolean))
  (Default|Levitate (.AsIllusion%20Player%20Controller (Utilities|Casting|CastToIllusion_PlayerController (Game|GetPlayerController 0))) self))

(fn ConstructionScript)